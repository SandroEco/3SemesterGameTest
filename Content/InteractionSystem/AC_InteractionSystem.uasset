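; Player controller component that tracks the interactable nearest the controlled pawn and forwards interaction requests to it.
; On BeginPlay it adds a hidden sphere to the pawn, overlapping only a configured object channel, and starts a looping timer.
; Update polls the sphere's overlaps to cache the closest actor within a fixed distance cap, clearing it otherwise.
; Interact sends an interface message to that cached actor, passing the controller.
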(event `self.ReceiveBeginPlay`
  (bind _asplayer_controller (cast `PlayerController` (`self.GetOwner`))
    (:`then`
      (bind _output_get (set `self.PCRef` _asplayer_controller))
      (bind _returnvalue (`|AddComponentByClass` :`self` (`Controller.K2_GetPawn` _output_get) :`Class` "/Script/Engine.SphereComponent"))
      (set `self.Collision` _returnvalue)
      (`SphereComponent.SetSphereRadius` (`self.Collision`) (`self.Sphere Radius`) true)
      (`PrimitiveComponent.SetCollisionResponseToAllChannels` (`self.Collision`) "ECR_Ignore")
      (`PrimitiveComponent.SetCollisionResponseToChannel` (`self.Collision`) (`self.ObjectChannel`) "ECR_Overlap")
      (`SceneComponent.SetHiddenInGame` (`self.Collision`) true false)
      (bind _returnvalue_2 (`KismetSystemLibrary.K2_SetTimerDelegate` (`|CreateDelegate` :!event `Update`) 0.1 true))
      (set `self.UpdateTimer` _returnvalue_2))
    (:`CastFailed`
      (`KismetSystemLibrary.PrintString` (`KismetStringLibrary.Concat_StrStr` (`KismetSystemLibrary.GetDisplayName` (`self.GetOwner`)) ": Is not a player controller.") true true (struct :`G` 0.66 :`B` 1.0 :`A` 1.0) 10.0))))

(event `OnBeginOverlapInteractable`
  (params (OverlappedComponent :type "PrimitiveComponent Object Reference") (OtherActor :type "Actor Object Reference") (OtherComp :type "PrimitiveComponent Object Reference") (OtherBodyIndex :type Integer) (bFromSweep :type Boolean) (SweepResult :type "HitResult Structure (by ref)")))

(event `OnEndOverlapInteractable`
  (params (OverlappedComponent :type "PrimitiveComponent Object Reference") (OtherActor :type "Actor Object Reference") (OtherComp :type "PrimitiveComponent Object Reference") (OtherBodyIndex :type Integer)))

(event `Interact`
  (params (PC :type "PlayerController Object Reference"))
  (bind _nearest_interactable (`self.Nearest Interactable`)
    (:`then`
      (message `/Game/InteractionSystem/I_Interact.Interact` _nearest_interactable PC))
    (:`else`)))

(fn `Update`
  (locals (_Distance :type "Float (double-precision)" :default 1000.0))
  (set `local._Distance` 1000.0)
  (for _array_element (`PrimitiveComponent.GetOverlappingActors` (`self.Collision`) null)
    (bind _returnvalue (`KismetMathLibrary.Vector_Distance` (`Actor.K2_GetActorLocation` _array_element) (`SceneComponent.K2_GetComponentLocation` (`self.Collision`))))
    (if (< _returnvalue (`local._Distance`))
      (set `self.Nearest Interactable` _array_element)
      (set `local._Distance` _returnvalue)))
  (if (>= (`local._Distance`) 1000.0)
    (set `self.Nearest Interactable` null)))