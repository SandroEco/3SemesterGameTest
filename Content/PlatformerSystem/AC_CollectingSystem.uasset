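; Actor component in the platformer system that keeps the count of collected carrots.
; The AddCarrot event raises the count and caps it at MaxCarrots, while the Remove event lowers it and stops it at zero.
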(event `AddCarrot`
  (params (Amount :type Integer))
  (bind _output_get (set `self.Carrots` (+ (stale _output_get) Amount)))
  (if (> (`self.Carrots`) (`self.MaxCarrots`))
    (set `self.Carrots` (`self.MaxCarrots`))))

(event `Remove`
  (params (Amount :type Integer))
  (bind _output_get (set `self.Carrots` (- (stale _output_get) Amount)))
  (if (< (`self.Carrots`) 0)
    (set `self.Carrots` 0)))