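; BP_Ears is a spline-mesh actor that stretches between a reference component and a target point, apparently as a hook-like ear.
; SetPoints runs the Hook timeline to extend the mesh end toward the target, while Reverse runs a second timeline to retract it.
; Both convert world positions into actor-local space for the spline mesh.
; Once either timeline has updated, Tick keeps the start pinned to the moving reference component.
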(event `self.ReceiveTick`
  (params (DeltaSeconds :type "Float (single-precision)"))
  (if (`self.bSpawned`)
    (`SplineMeshComponent.SetStartPosition` (`self.SplineMeshComponent`) (`KismetMathLibrary.InverseTransformLocation` (`self.GetTransform`) (`SceneComponent.K2_GetComponentLocation` (`self.Empty Ref`))) true)))

(event `SetPoints`
  (params (EndPoint :type "Vector Structure") (EmptyRef :type "StaticMeshComponent Object Reference"))
  (bind _returnvalue (`self.GetTransform`))
  (bind _returnvalue_2 (`KismetMathLibrary.InverseTransformLocation` _returnvalue (`SceneComponent.K2_GetComponentLocation` EmptyRef)))
  (set `self.Empty Ref` EmptyRef)
  (bind (_direction _alpha) (`Timeline|Hook` :!via `PlayFromStart`)
    (:`Update`
      (`SplineMeshComponent.SetStartAndEnd` (`self.SplineMeshComponent`) _returnvalue_2 (0.0 0.0 0.0) (`KismetMathLibrary.VLerp` _returnvalue_2 (`KismetMathLibrary.InverseTransformLocation` _returnvalue EndPoint) _alpha) (0.0 0.0 0.0) true)
      (set `self.bSpawned` true))))

(event `Reverse`
  (params (EndPoint :type "Vector Structure") (EmptyRef :type "StaticMeshComponent Object Reference"))
  (bind _returnvalue (`self.GetTransform`))
  (bind _returnvalue_2 (`KismetMathLibrary.InverseTransformLocation` _returnvalue (`SceneComponent.K2_GetComponentLocation` EmptyRef)))
  (set `self.Empty Ref` EmptyRef)
  (bind (_direction _alpha) (`Timeline|Timeline` :!via `PlayFromStart`)
    (:`Update`
      (`SplineMeshComponent.SetStartAndEnd` (`self.SplineMeshComponent`) _returnvalue_2 (0.0 0.0 0.0) (`KismetMathLibrary.VLerp` (`KismetMathLibrary.InverseTransformLocation` _returnvalue EndPoint) _returnvalue_2 _alpha) (0.0 0.0 0.0) true)
      (set `self.bSpawned` true))))

(fn `UserConstructionScript`)